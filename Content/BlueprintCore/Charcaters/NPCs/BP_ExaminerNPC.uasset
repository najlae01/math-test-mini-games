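; BP_ExaminerNPC is an examiner NPC that the player can talk to in order to start a test.
; Player overlap with its collision box shows an interact widget, which turns on its yaw to face the player while no conversation is active.
; Clicking its button opens the dialogue widget, hides the prompt and calls StartTestOnInteraction.
; When the player leaves the box, both widgets are cleared and the talking state resets.
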(event OnComponentBeginOverlap(CollisionBox)
  (params (OverlappedComponent :type Primitive%20Component%20Object%20Reference) (OtherActor :type Actor%20Object%20Reference) (OtherComp :type Primitive%20Component%20Object%20Reference) (OtherBodyIndex :type Integer) (bFromSweep :type Boolean) (SweepResult :type Hit%20Result%20Structure%20%28by%20ref%29))
  (if (Actor|ActorHasTag OtherActor "Player")
    (Development|PrintString "Hello")
    (if (not (Variables|Default|GetIsTalkingToPlayer))
      (Rendering|SetVisibility (Variables|Default|GetInteractWidget) true false))
    (else
      (Variables|Default|SetIsTalkingToPlayer false))))

(event OnComponentEndOverlap(CollisionBox)
  (params (OverlappedComponent :type Primitive%20Component%20Object%20Reference) (OtherActor :type Actor%20Object%20Reference) (OtherComp :type Primitive%20Component%20Object%20Reference) (OtherBodyIndex :type Integer))
  (if (Actor|ActorHasTag OtherActor "Player")
    (Variables|Default|SetIsTalkingToPlayer false)
    (bind _npcdialoguewidget (Variables|Default|GetNpcDialogueWidget)
      (:then
        (Widget|RemovefromParent _npcdialoguewidget))
      (:else
        _))
    (Rendering|SetVisibility (Variables|Default|GetInteractWidget) false false)))

(event Custom|OnClicked_Event
  (Variables|Default|SetIsTalkingToPlayer true)
  (bind _returnvalue (UserInterface|CreateWidget "/Game/Widgets/WBP_NPC_Dialogue.WBP_NPC_Dialogue_C" (Game|GetPlayerController 0)))
  (UserInterface|Viewport|AddtoViewport _returnvalue 2)
  (Variables|Default|SetNpcDialogueWidget _returnvalue)
  (Rendering|SetVisibility (Variables|Default|GetInteractWidget) false false)
  (Class|ExaminerNPC|StartTestonInteraction))

(event EventBeginPlay
  (bind _aswbp_interact_npc (Utilities|Casting|CastToWBP_Interact_NPC (UserInterface|GetWidget (Variables|Default|GetInteractWidget))))
  (bind _output_get (Variables|Default|SetInteractNPCWidget _aswbp_interact_npc))
  (EventDispatchers|AssignOnClicked (Variables|/Game/Widgets/WBP_Interact_NPC.WBP_Interact_NPC_C|GetInteractButton _output_get) (delegate Custom|OnClicked_Event)))

(event Collision|EventActorBeginOverlap
  (params (OtherActor :type Actor%20Object%20Reference)))

(event EventTick
  (params (DeltaSeconds :type Float%20%28single-precision%29))
  (bind _interactwidget (Variables|Default|GetInteractWidget))
  (if (not (Variables|Default|GetIsTalkingToPlayer))
    (Transformation|SetWorldRotation _interactwidget (Math|Rotator|MakeRotator 0.0 0.0 (.yaw (Math|Rotator|FindLookatRotation (Transformation|GetWorldLocation _interactwidget) (Transformation|GetActorLocation (Game|GetPlayerCharacter 0))))) false false)))

(fn ConstructionScript)