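; BP_MathoriaHUD is the HUD that shows the splash screen on BeginPlay and routes the player onward from its tap-to-play button.
; With a valid current user and a true OnSplashScreen result from the player state, it collapses the splash and opens the overlay.
; Otherwise it opens the QR reader, passing it the splash widget.
; Unconnected leftovers remain for a handwriting test, older email-verified authentication and Game level streaming visibility.
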(event Custom|OnClicked_Event
  (Utilities|IsValid (Class|AuthMiscLibrary|CurrentUser)
    (:Is%20Valid
      (bind _asbp_mathoria_player_state (Utilities|Casting|CastToBP_MathoriaPlayerState (Game|GetPlayerState 0)))
      (bind _returnvalue (Class|MathoriaPlayerState|OnSplashScreen _asbp_mathoria_player_state))
      (if _returnvalue
        (Widget|SetVisibility (Variables|Default|GetSplashScreenRef) "Collapsed")
        (bind _returnvalue_2 (UserInterface|CreateWidget "/Game/Widgets/WBP_Overlay.WBP_Overlay_C" (Game|GetPlayerController 0) (Variables|Default|GetSplashScreenRef)))
        (UserInterface|Viewport|AddtoViewport _returnvalue_2 4)
        (else
          (bind _returnvalue_3 (UserInterface|CreateWidget "/Game/Widgets/WBP_QrReader.WBP_QrReader_C" (Game|GetPlayerController 0) (Variables|Default|GetSplashScreenRef) :!label _label))
          (UserInterface|Viewport|AddtoViewport _returnvalue_3 4))))
    (:Is%20Not%20Valid
      (goto _label))))

(event EventBeginPlay
  (bind _returnvalue (UserInterface|CreateWidget "/Game/Widgets/WBP_SplashSreen.WBP_SplashSreen_C" (Game|GetPlayerController 0)))
  (UserInterface|Viewport|AddtoViewport _returnvalue 2)
  (bind _output_get (Variables|Default|SetSplashScreenRef _returnvalue))
  (EventDispatchers|AssignOnClicked (Variables|/Game/Widgets/WBP_SplashSreen.WBP_SplashSreen_C|GetTapToPlayButton _output_get) (delegate Custom|OnClicked_Event)))

(fn ConstructionScript)